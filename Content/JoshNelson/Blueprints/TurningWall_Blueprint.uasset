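; Turning wall actor that rotates smoothly in yaw through a list of preset angles.
; Construction sets the initial target to the actor's current yaw, and Tick interpolates rotation toward the target yaw at RotateSpeed with RInterpTo, zeroing pitch and roll.
; NewRotationTarget takes the next angle from RotationTargets and advances a wrapping index; nothing in this Blueprint calls it.
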(event EventBeginPlay)

(event Collision|EventActorBeginOverlap
  (params (OtherActor :type Actor%20Object%20Reference)))

(event EventTick
  (params (DeltaSeconds :type Float%20%28single-precision%29))
  (Transformation|SetActorRotation (Math|Interpolation|RInterpTo (Transformation|GetActorRotation) (Math|Rotator|MakeRotator 0.0 0.0 (Variables|Default|GettargetRotation)) (Utilities|Time|GetWorldDeltaSeconds) (Variables|Default|GetRotateSpeed))))

(fn ConstructionScript
  (Variables|Default|SettargetRotation (.Yaw (Math|Vector|GetYawPitchfromVector (Math|Rotator|GetRotationXVector (Transformation|GetActorRotation))))))

(fn NewRotationTarget
  (Math|Integer|CompareInt (Variables|Default|GettargetIndex) (Utilities|Array|Length (Variables|Default|GetrotationTargets))
    (:<
      (Variables|Default|SettargetRotation (Utilities|Array|Get(acopy) (Variables|Default|GetrotationTargets) (Variables|Default|GettargetIndex)))
      (bind _result (Math|Integer|IncrementInt (Variables|Default|GettargetIndex))
        (:%20%20
          (Variables|Default|SettargetIndex (Math|Integer|%(Integer) _result (Utilities|Array|Length (Variables|Default|GetrotationTargets)))))))))