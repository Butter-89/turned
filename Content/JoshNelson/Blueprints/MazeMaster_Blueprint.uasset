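; MazeMaster is a maze controller that periodically turns a random wall and aims a lightning beam effect at it.
; Its construction script caches all TurningWall_Blueprint actors and performs an initial turn.
; Tick accumulates time and calls TurnWall whenever the delay is exceeded.
; TurnWall asks a random cached wall for a new rotation target and points three PLightning beam emitters at that wall's location.
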(event EventBeginPlay)

(event Collision|EventActorBeginOverlap
  (params (OtherActor :type Actor%20Object%20Reference)))

(event EventTick
  (params (DeltaSeconds :type Float%20%28single-precision%29))
  (bind _output_get (Variables|Default|SetwallTurnTimer (+ DeltaSeconds (Variables|Default|GetwallTurnTimer))))
  (Math|Float|CompareFloat _output_get (Variables|Default|GetwallTurnDelay)
    (:>
      (Variables|Default|SetwallTurnTimer 0.0)
      (CallFunction|TurnWall))))

(fn ConstructionScript
  (bind _outactors (Actor|GetAllActorsOfClass "/Game/JoshNelson/Blueprints/TurningWall_Blueprint.TurningWall_Blueprint_C"))
  (Variables|Default|Setwalls _outactors)
  (CallFunction|TurnWall))

(fn TurnWall
  (bind _p_lightning (Variables|Default|Getp_lightning))
  (bind _output_get (LocalVariables|SetNewLocalVar_1 (Utilities|Array|Get(acopy) (Variables|Default|Getwalls) (Math|Random|RandomIntegerinRange 0 (- (Utilities|Array|Length (Variables|Default|Getwalls)) 1)))))
  (Default|NewRotationTarget _output_get)
  (Class|ParticleSystemComponent|SetBeamTargetPoint _p_lightning 0 (Transformation|GetActorLocation _output_get))
  (Class|ParticleSystemComponent|SetBeamTargetPoint _p_lightning 1 (Transformation|GetActorLocation _output_get))
  (Class|ParticleSystemComponent|SetBeamTargetPoint _p_lightning 2 (Transformation|GetActorLocation _output_get)))