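; GravityWall is a wall actor whose Box trigger switches a WallWalkerCharacter in and out of wall running.
; On begin overlap, a character moving above a small speed threshold and not already wall running gets WallRunning set and its location stored as WallPosition.
; On end overlap, WallRunning clears and the character's rotation resets to zero.
; Disconnected nodes hold unused attempts to rotate the player from the wall's orientation.
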(event OnComponentBeginOverlap(Box)
  (params (OverlappedComponent :type Primitive%20Component%20Object%20Reference) (OtherActor :type Actor%20Object%20Reference) (OtherComp :type Primitive%20Component%20Object%20Reference) (OtherBodyIndex :type Integer) (bFromSweep :type Boolean) (SweepResult :type Hit%20Result%20Structure%20%28by%20ref%29))
  ;[1 1 1] Enabling wall running state
  (bind _aswall_walker_character (Utilities|Casting|CastToWallWalkerCharacter OtherActor))
  (if (not (Variables|/Game/ThirdPersonBP/Xiubo/Blueprints/WallWalkerCharacter.WallWalkerCharacter_C|GetwallRunning _aswall_walker_character))
    (if (> (Math|Vector|VectorLength (Transformation|GetVelocity _aswall_walker_character)) 5e+01)
      (Variables|/Game/ThirdPersonBP/Xiubo/Blueprints/WallWalkerCharacter.WallWalkerCharacter_C|SetwallRunning _aswall_walker_character true)
      (Variables|/Game/ThirdPersonBP/Xiubo/Blueprints/WallWalkerCharacter.WallWalkerCharacter_C|SetwallPosition _aswall_walker_character (Transformation|GetActorLocation _aswall_walker_character)))))

(event OnComponentEndOverlap(Box)
  (params (OverlappedComponent :type Primitive%20Component%20Object%20Reference) (OtherActor :type Actor%20Object%20Reference) (OtherComp :type Primitive%20Component%20Object%20Reference) (OtherBodyIndex :type Integer))
  ;[1 1 1] Disabling wall running state
  (bind _aswall_walker_character (Utilities|Casting|CastToWallWalkerCharacter OtherActor))
  (Variables|/Game/ThirdPersonBP/Xiubo/Blueprints/WallWalkerCharacter.WallWalkerCharacter_C|SetwallRunning _aswall_walker_character false)
  (Transformation|SetActorRotation _aswall_walker_character))

(fn ConstructionScript)